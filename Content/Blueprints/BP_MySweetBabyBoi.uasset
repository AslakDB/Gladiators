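; Player character Blueprint that plays combat and pickup animations and shows a blood hit screen on damage.
; Light and heavy attack inputs pick sword, axe or spear montages from weapon flags; attacks and dodge require being alive.
; Use input plays pickup montages when near a weapon or potion.
; Each action's DoOnce resets after a montage-length Delay to prevent retriggering, and TakenDamage creates the hit widget lazily, then reuses it.
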(event Input|EnhancedActionEvents|EnhancedInputActionUseInput
  (params (ActionValue :type Boolean) (ElapsedSeconds :type Float%20%28double-precision%29) (TriggeredSeconds :type Float%20%28double-precision%29) (InputAction :type Input%20Action%20Object%20Reference :default "/Game/input/UseInput.UseInput"))
  (:Started
    (if (Variables|Default|GetCloseToSpear)
      (Utilities|FlowControl|DoOnce false :!label _label
        (:Completed
          (bind _returnvalue (Animation|PlayAnimMontage "/Game/Main_Character/Animation/AS_MC_Pickup_1__Montage.AS_MC_Pickup_1__Montage" 1.5 "None"))
          (Utilities|FlowControl|Delay _returnvalue)
          (goto _label Reset))))))

(event Input|EnhancedActionEvents|EnhancedInputActionDodgeInput
  (params (ActionValue :type Float%20%28double-precision%29) (ElapsedSeconds :type Float%20%28double-precision%29) (TriggeredSeconds :type Float%20%28double-precision%29) (InputAction :type Input%20Action%20Object%20Reference :default "/Game/input/DodgeInput.DodgeInput"))
  (:Started
    (if (Variables|Default|GetIsAlive)
      (Utilities|FlowControl|DoOnce false :!label _label
        (:Completed
          (bind _returnvalue (Animation|PlayAnimMontage "/Game/Main_Character/Animation/AS_MC_Dodge_Montage.AS_MC_Dodge_Montage" 1.0 "None"))
          (Utilities|FlowControl|Delay _returnvalue)
          (goto _label Reset))))))

(event Input|EnhancedActionEvents|EnhancedInputActionUseInput
  (params (ActionValue :type Boolean) (ElapsedSeconds :type Float%20%28double-precision%29) (TriggeredSeconds :type Float%20%28double-precision%29) (InputAction :type Input%20Action%20Object%20Reference :default "/Game/input/UseInput.UseInput"))
  (:Started
    (if (Variables|Default|GetCloseToPotion)
      (Utilities|FlowControl|DoOnce false :!label _label
        (:Completed
          (bind _returnvalue (Animation|PlayAnimMontage "/Game/Main_Character/Animation/AS_MC_PickupNew_Montage.AS_MC_PickupNew_Montage" 2.0 "None"))
          (Utilities|FlowControl|Delay _returnvalue)
          (goto _label Reset))))))

(event Input|EnhancedActionEvents|EnhancedInputActionUseInput
  (params (ActionValue :type Boolean) (ElapsedSeconds :type Float%20%28double-precision%29) (TriggeredSeconds :type Float%20%28double-precision%29) (InputAction :type Input%20Action%20Object%20Reference :default "/Game/input/UseInput.UseInput"))
  (:Started
    (if (Variables|Default|GetCloseToSword)
      (Utilities|FlowControl|DoOnce false :!label _label
        (:Completed
          (bind _returnvalue (Animation|PlayAnimMontage "/Game/Main_Character/Animation/AS_MC_PickupNew_Montage.AS_MC_PickupNew_Montage" 2.0 "None"))
          (Utilities|FlowControl|Delay _returnvalue)
          (goto _label Reset))))))

(event Input|EnhancedActionEvents|EnhancedInputActionAttackInput
  (params (ActionValue :type Float%20%28double-precision%29) (ElapsedSeconds :type Float%20%28double-precision%29) (TriggeredSeconds :type Float%20%28double-precision%29) (InputAction :type Input%20Action%20Object%20Reference :default "/Game/input/AttackInput.AttackInput"))
  (:Started
    (if (Variables|Default|GetHaveSword)
      (if (Variables|Default|GetIsAlive)
        (Utilities|FlowControl|DoOnce false :!label _label
          (:Completed
            (bind _returnvalue (Animation|PlayAnimMontage "/Game/Main_Character/Animation/Attacks/AS_MC_SwordAttack_Light_1__Montage.AS_MC_SwordAttack_Light_1__Montage" 1.0 "None"))
            (Utilities|FlowControl|Delay _returnvalue)
            (goto _label Reset)))))))

(event Input|EnhancedActionEvents|EnhancedInputActionAttackInput
  (params (ActionValue :type Float%20%28double-precision%29) (ElapsedSeconds :type Float%20%28double-precision%29) (TriggeredSeconds :type Float%20%28double-precision%29) (InputAction :type Input%20Action%20Object%20Reference :default "/Game/input/AttackInput.AttackInput"))
  (:Started
    (if (Variables|Default|GetHaveAxe)
      (if (Variables|Default|GetIsAlive)
        (Utilities|FlowControl|DoOnce false :!label _label
          (:Completed
            (bind _returnvalue (Animation|PlayAnimMontage "/Game/Main_Character/Animation/Attacks/AS_MC_AxeAttack_Light_1__Montage.AS_MC_AxeAttack_Light_1__Montage" 1.0 "None"))
            (Utilities|FlowControl|Delay _returnvalue)
            (goto _label Reset)))))))

(event Input|EnhancedActionEvents|EnhancedInputActionAttackInput
  (params (ActionValue :type Float%20%28double-precision%29) (ElapsedSeconds :type Float%20%28double-precision%29) (TriggeredSeconds :type Float%20%28double-precision%29) (InputAction :type Input%20Action%20Object%20Reference :default "/Game/input/AttackInput.AttackInput"))
  (:Started
    (if (Variables|Default|GetHaveSpear)
      (if (Variables|Default|GetIsAlive)
        (Utilities|FlowControl|DoOnce false :!label _label
          (:Completed
            (bind _returnvalue (Animation|PlayAnimMontage "/Game/Main_Character/Animation/Attacks/AS_MC_SpearAttack_Light_1__Montage.AS_MC_SpearAttack_Light_1__Montage" 1.0 "None"))
            (Utilities|FlowControl|Delay _returnvalue)
            (goto _label Reset)))))))

(event Input|EnhancedActionEvents|EnhancedInputActionHeavyAttackInput
  (params (ActionValue :type Float%20%28double-precision%29) (ElapsedSeconds :type Float%20%28double-precision%29) (TriggeredSeconds :type Float%20%28double-precision%29) (InputAction :type Input%20Action%20Object%20Reference :default "/Game/input/HeavyAttackInput.HeavyAttackInput"))
  (:Started
    (if (Variables|Default|GetHaveSword)
      (if (Variables|Default|GetIsAlive)
        (Utilities|FlowControl|DoOnce false :!label _label
          (:Completed
            (bind _returnvalue (Animation|PlayAnimMontage "/Game/Main_Character/Animation/Attacks/AS_MC_SwordAttack_Heavy_3__Montage.AS_MC_SwordAttack_Heavy_3__Montage" 1.0 "None"))
            (Utilities|FlowControl|Delay _returnvalue)
            (goto _label Reset)))))))

(event Input|EnhancedActionEvents|EnhancedInputActionHeavyAttackInput
  (params (ActionValue :type Float%20%28double-precision%29) (ElapsedSeconds :type Float%20%28double-precision%29) (TriggeredSeconds :type Float%20%28double-precision%29) (InputAction :type Input%20Action%20Object%20Reference :default "/Game/input/HeavyAttackInput.HeavyAttackInput"))
  (:Started
    (if (Variables|Default|GetHaveAxe)
      (if (Variables|Default|GetIsAlive)
        (Utilities|FlowControl|DoOnce false :!label _label
          (:Completed
            (bind _returnvalue (Animation|PlayAnimMontage "/Game/Main_Character/Animation/Attacks/AS_MC_AxeAttack_Heavy_1__Montage.AS_MC_AxeAttack_Heavy_1__Montage" 1.0 "None"))
            (Utilities|FlowControl|Delay _returnvalue)
            (goto _label Reset)))))))

(event Input|EnhancedActionEvents|EnhancedInputActionHeavyAttackInput
  (params (ActionValue :type Float%20%28double-precision%29) (ElapsedSeconds :type Float%20%28double-precision%29) (TriggeredSeconds :type Float%20%28double-precision%29) (InputAction :type Input%20Action%20Object%20Reference :default "/Game/input/HeavyAttackInput.HeavyAttackInput"))
  (:Started
    (if (Variables|Default|GetHaveSpear)
      (if (Variables|Default|GetIsAlive)
        (Utilities|FlowControl|DoOnce false :!label _label
          (:Completed
            (bind _returnvalue (Animation|PlayAnimMontage "/Game/Main_Character/Animation/Attacks/AS_MC_SpearAttack_Heavy_1__Montage.AS_MC_SpearAttack_Heavy_1__Montage" 1.0 "None"))
            (Utilities|FlowControl|Delay _returnvalue)
            (goto _label Reset)))))))

(event Input|EnhancedActionEvents|EnhancedInputActionUseInput
  (params (ActionValue :type Boolean) (ElapsedSeconds :type Float%20%28double-precision%29) (TriggeredSeconds :type Float%20%28double-precision%29) (InputAction :type Input%20Action%20Object%20Reference :default "/Game/input/UseInput.UseInput"))
  (:Started
    (if (Variables|Default|GetCloseToAxe)
      (Utilities|FlowControl|DoOnce false :!label _label
        (:Completed
          (bind _returnvalue (Animation|PlayAnimMontage "/Game/Main_Character/Animation/AS_MC_Pickup_1__Montage.AS_MC_Pickup_1__Montage" 1.5 "None"))
          (Utilities|FlowControl|Delay _returnvalue)
          (goto _label Reset))))))

(event EventTakenDamage
  ;[1 1 1] HitScreen
  (Variables|Default|GetBloodHitWidget
    (:then
      (Default|PlayHitAnimation (Variables|Default|GetBloodHitWidget)))
    (:else
      (bind _returnvalue (UserInterface|CreateWidget "/Game/HUD/BP_HitScreen.BP_HitScreen_C" (Game|GetPlayerController 0)))
      (bind _output_get (Variables|Default|SetBloodHitWidget _returnvalue))
      (UserInterface|Viewport|AddtoViewport _output_get 0)
      (Default|PlayHitAnimation (Variables|Default|GetBloodHitWidget)))))

(fn ConstructionScript)