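; Test sword Blueprint that attaches a Niagara slash trail to its skeletal mesh.
; On BeginPlay it spawns SlashTestTrail at the midpoint of the Trail_Top and Trail_Bottom sockets, with its Z axis along the line between them.
; The distance between the sockets sets the system's TrailWidth parameter once at spawn, so the trail matches that span.
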(event EventBeginPlay
  (bind _skeletalmesh (Variables|Default|GetSkeletalMesh))
  (bind _returnvalue (Transformation|GetSocketLocation _skeletalmesh "Trail_Top"))
  (bind _returnvalue_2 (Transformation|GetSocketLocation _skeletalmesh "Trail_Bottom"))
  (bind _returnvalue_3 (- _returnvalue _returnvalue_2))
  (|CallParentFunction)
  (Utilities|FlowControl|Sequence
    (:then_0
      (bind _returnvalue_4 (Niagara|SpawnSystemAttached "/Game/NiagaraVFX/SlashTrailTest/SlashTestTrail.SlashTestTrail" _skeletalmesh "None" (/ (+ _returnvalue _returnvalue_2) 2.0) (Math|Rotator|MakeRotfromZ _returnvalue_3) "KeepWorldPosition" false))
      (Effects|Components|ParticleSystem|SetFloatParameter _returnvalue_4 "TrailWidth" (Math|Vector|VectorLength _returnvalue_3)))))

(event Collision|EventActorBeginOverlap
  (params (OtherActor :type Actor%20Object%20Reference)))

(event EventTick
  (params (DeltaSeconds :type Float%20%28single-precision%29)))

(fn ConstructionScript)