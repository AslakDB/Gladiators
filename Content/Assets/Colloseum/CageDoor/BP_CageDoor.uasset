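; BP_CageDoor is a Colosseum cage door the player opens and closes with E after stepping through instructional dialogue.
; Overlap volumes show an interact prompt and, for BP_MySweetBabyBoi only, enable input and open a Gate node.
; Each press advances a dialogue widget with a sound; once lines run out, presses remove it and pass the Gate to a FlipFlop.
; The FlipFlop plays or reverses a Timeline that lerps the mesh's height.
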(event OnComponentBeginOverlap(Trigger)
  (params (OverlappedComponent :type Primitive%20Component%20Object%20Reference) (OtherActor :type Actor%20Object%20Reference) (OtherComp :type Primitive%20Component%20Object%20Reference) (OtherBodyIndex :type Integer) (bFromSweep :type Boolean) (SweepResult :type Hit%20Result%20Structure%20%28by%20ref%29))
  ;[1 1 1] Gate Opens and closes if actor close enough
  (Utilities|Casting|CastToBP_MySweetBabyBoi OtherActor)
  (Input|EnableInput (Game|GetPlayerController 0))
  (Utilities|FlowControl|Gate true) ; enters at Open
)

(event OnComponentEndOverlap(Trigger)
  (params (OverlappedComponent :type Primitive%20Component%20Object%20Reference) (OtherActor :type Actor%20Object%20Reference) (OtherComp :type Primitive%20Component%20Object%20Reference) (OtherBodyIndex :type Integer))
  ;[1 1 1] Gate Opens and closes if actor close enough
  (Utilities|Casting|CastToBP_MySweetBabyBoi OtherActor)
  (Input|DisableInput (Game|GetPlayerController 0))
  (Utilities|FlowControl|Gate true) ; enters at Close
)

(event OnComponentBeginOverlap(Text)
  (params (OverlappedComponent :type Primitive%20Component%20Object%20Reference) (OtherActor :type Actor%20Object%20Reference) (OtherComp :type Primitive%20Component%20Object%20Reference) (OtherBodyIndex :type Integer) (bFromSweep :type Boolean) (SweepResult :type Hit%20Result%20Structure%20%28by%20ref%29))
  ;[1 1 1] Interact Text appears when player close enough
  (Utilities|Casting|CastToBP_MySweetBabyBoi OtherActor)
  (Development|SetHiddeninGame (Variables|Default|GetWidget) false false))

(event OnComponentEndOverlap(Text)
  (params (OverlappedComponent :type Primitive%20Component%20Object%20Reference) (OtherActor :type Actor%20Object%20Reference) (OtherComp :type Primitive%20Component%20Object%20Reference) (OtherBodyIndex :type Integer))
  ;[1 1 1] Interact Text appears when player close enough
  (Utilities|Casting|CastToBP_MySweetBabyBoi OtherActor)
  (Development|SetHiddeninGame (Variables|Default|GetWidget) true false))

(event Input|KeyboardEvents|E
  (params (Key :type Key%20Structure :default "None"))
  ;[1 1 1] Gate Opens and closes if actor close enough
  (:Pressed
    (Utilities|FlowControl|Sequence
      (:then_0
        ;[1 1 1] Dialouge Instructional Text
        (CallFunction|Talk)
        (Math|Integer|IncrementInt (Variables|Default|GetTalkIndex)
          (:%20%20
            (if (< (Variables|Default|GetTalkIndex) (Utilities|Array|Length (Variables|Default|GetDialouge)))
              (Variables|Default|GetUI
                (:then
                  _)
                (:else
                  (bind _returnvalue (UserInterface|CreateWidget "/Game/Assets/Colloseum/CageDoor/BP_Dialouge.BP_Dialouge_C" (Game|GetPlayerController 0)))
                  (bind _output_get (Variables|Default|SetUI _returnvalue))
                  (UserInterface|Viewport|AddtoViewport _output_get 0)))
              (Rendering|Components|TextRender|SetText (Variables|/Game/Assets/Colloseum/CageDoor/BP_Dialouge.BP_Dialouge_C|GetDialouge (Variables|Default|GetUI)) (Utilities|Text|ToText(String) (Utilities|Array|Get(acopy) (Variables|Default|GetDialouge) (Variables|Default|GetTalkIndex))))
              (Audio|PlaySound2D "/Engine/VREditor/Sounds/UI/Camera_Shutter.Camera_Shutter" 1.0 1.0 0.0 0 0)
              (else
                (Widget|RemovefromParent (Variables|Default|GetUI))
                (Utilities|FlowControl|Gate true
                  (:Exit
                    (Utilities|FlowControl|FlipFlop
                      (:A
                        (bind _cagedooropen (Timeline|Timeline Play)
                          (:Update
                            (Transformation|SetRelativeLocation (Variables|Default|GetStaticMesh) (Math|Vector|MakeVector 0.0 0.0 (Math|Float|Lerp (Variables|Default|GetClosedGate) (Variables|Default|GetOpenGate) _cagedooropen)) false false))))
                      (:B
                        (Timeline|Timeline Reverse)))))))))))))

(fn ConstructionScript)